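; VR player character that records, recognizes and displays motion gestures through the right controller's VRGestureRecognition component.
; Thumbstick records a gesture under an incrementing ID, grip clears all gestures, and trigger listens until release or a match, which prints its ID.
; After recording or clearing, CreateSpline replaces GestureDisplayBP to draw all templates as splines at a point computed from SteamVR chaperone bounds at BeginPlay.
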(event `Key|Escape`
  (params (Key :type "Key Structure" :default "AnyKey"))
  (:`Pressed`
    (`KismetSystemLibrary.QuitGame` null "Quit")))

(event `Key|MotionController_Right_Grip1`
  (params (Key :type "Key Structure" :default "AnyKey"))
  (:`Pressed`
    (`VRGestureRecognitionComponent.ClearGestures` (`self.VRGestureRecognitionRight`) :!label _label)
    (set `self.GestureCpt` 0)
    (`self.CreateSpline`)))

(event `Key|MotionController_Right_Grip2`
  (params (Key :type "Key Structure" :default "AnyKey"))
  (:`Pressed`
    (goto _label)))

(event `Key|MotionController_Right_Trigger`
  (params (Key :type "Key Structure" :default "AnyKey"))
  (bind _vrgesturerecognitionright (`self.VRGestureRecognitionRight`))
  (:`Pressed`
    (`VRGestureRecognitionComponent.ListenAllGestures` _vrgesturerecognitionright))
  (:`Released`
    (`VRGestureRecognitionComponent.StopListenGesture` _vrgesturerecognitionright)))

(event `Key|MotionController_Right_Thumbstick`
  (params (Key :type "Key Structure" :default "AnyKey"))
  (bind _vrgesturerecognitionright (`self.VRGestureRecognitionRight`))
  ;[1 1 1] Record gesture on thumbstick press
  (:`Pressed`
    (`VRGestureRecognitionComponent.RecordGesture` _vrgesturerecognitionright (`self.GestureCpt`)))
  (:`Released`
    (`VRGestureRecognitionComponent.StopRecordGesture` _vrgesturerecognitionright)
    (`self.CreateSpline`)
    (`/Engine/EditorBlueprintResources/StandardMacros.IncrementInt` (`self.GestureCpt`))))

(event `self.ReceiveBeginPlay`
  (bind _returnvalue (`SteamVRChaperoneComponent.GetBounds` (`self.SteamVRChaperone`)))
  (`HeadMountedDisplayFunctionLibrary.EnableHMD` true)
  ;[1 1 1] Bind event to OnGestureActivated
  (add `VRGestureRecognizer.OnGestureActivated` (`VRGestureRecognitionComponent.GestureRecognizer` (`self.VRGestureRecognitionRight`)) (delegate `OnGestureActivatedEvent`))
  (bind _outactors (`GameplayStatics.GetAllActorsOfClass` "/Game/GestureDisplay/DisplayPosition.DisplayPosition_C"))
  (set `self.GestureDisplayST` (`KismetMathLibrary.MakeTransform` (`KismetMathLibrary.MakeVector` (/ (+ (.x (`KismetArrayLibrary.Array_Get` _returnvalue)) (.x (`KismetArrayLibrary.Array_Get` _returnvalue 2))) 2.0) (/ (+ (.y (`KismetArrayLibrary.Array_Get` _returnvalue)) (.y (`KismetArrayLibrary.Array_Get` _returnvalue 2))) 2.0) 150.0))))

(event `OnGestureActivatedEvent`
  (params (GestureID :type Integer))
  ;[1 1 1] Bind event to OnGestureActivated
  (`KismetSystemLibrary.PrintString` (`KismetStringLibrary.Concat_StrStr` "Gesture Activated: " (`KismetStringLibrary.Conv_IntToString` GestureID)))
  (`VRGestureRecognitionComponent.StopListenGesture` (`self.VRGestureRecognitionRight`)))

(fn `CreateSpline`
  (bind _gesturemanager (`VRGestureRecognizer.GestureManager` (`VRGestureRecognitionComponent.GestureRecognizer` (`self.VRGestureRecognitionRight`))))
  (bind _outactors (`GameplayStatics.GetAllActorsOfClass` "/Game/GestureDisplay/GestureDisplayBP.GestureDisplayBP_C"))
  (for _array_element _outactors
    (`self.K2_DestroyActor` _array_element))
  (bind _returnvalue (`|SpawnActorFromClass` "/Game/GestureDisplay/GestureDisplayBP.GestureDisplayBP_C" (`self.GestureDisplayST`) "Undefined" "OverrideRootScale"))
  (bind _returnvalue_2 (`VRGestureTemplateManager.GetAllTemplates` _gesturemanager))
  (`/Game/GestureDisplay/GestureDisplayBP.CreateSplines` _returnvalue _returnvalue_2 _gesturemanager))

(fn `UserConstructionScript`)